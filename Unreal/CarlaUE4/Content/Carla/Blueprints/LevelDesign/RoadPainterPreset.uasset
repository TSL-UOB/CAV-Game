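; Road painter preset Blueprint for CARLA level design that scatters decals and static meshes along the map's roads.
; Construction creates a brush material instance and loads the current OpenDRIVE map, which supplies waypoint transforms.
; Spawn events place configured counts at random waypoints with randomized offset, yaw and scale.
; SetBlueprintVariables fills decal settings from DecalPropertiesConfig; the paint-over-time Tick branch is empty.
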(event `Spawn Meshes`
  (bind _random_offset_ (`self.Random Offset `))
  (bind _returnvalue (`KismetMathLibrary.RandomFloatInRange` (* _random_offset_ -1.0) _random_offset_))
  ;[1 1 1] Spawn meshes.
  (bind _returnvalue1 (`self.Load Waypoins from OD (Transform)` 500.0 :!label _label))
  (for (_ _array_index) (`self.Meshes Spawn`)
    (bind (_meshes _numberofmeshes) (break `/Game/Carla/Blueprints/LevelDesign/RoadPaintMeshes` (`|GetArrayItem` (`self.Meshes Spawn`) _array_index)))
    (for _ (range 1 (+ _numberofmeshes 1))
      (bind _returnvalue_2 (`self.Get any random points in the road` _returnvalue1))
      (bind _returnvalue_3 (`|SpawnActorFromClass` "/Script/Engine.StaticMeshActor" (`KismetMathLibrary.MakeTransform` (+ (+ (.location _returnvalue_2) (`KismetMathLibrary.MakeVector` _returnvalue _returnvalue)) (`self.Fixed mesh offset`)) (`KismetMathLibrary.MakeRotator` (.roll (.rotation _returnvalue_2)) (.pitch (.rotation _returnvalue_2)) (+ (`KismetMathLibrary.RandomFloatInRange` 0.0 (`self.Mesh Random Yaw`)) (.yaw (.rotation _returnvalue_2)))) (* (`self.Mesh scale`) (`KismetMathLibrary.RandomFloatInRange` (`self.Mesh min scale`) (`self.Mesh max scale`)))) "AdjustIfPossibleButDontSpawnIfColliding" "OverrideRootScale" null null))
      (`StaticMeshComponent.SetStaticMesh` (`StaticMeshActor.StaticMeshComponent` _returnvalue_3) _meshes))))

(event `self.SpawnMeshesEvent`
  ;[1 1 1] Spawn meshes.
  (goto _label))

(event `self.ReceiveTick`
  (params (DeltaSeconds :type "Float (single-precision)"))
  ;[1 1 1] Draw at tick
  (if (`self.Painting over time`)
    _))

(event `self.SetBlueprintVariables`
  (bind (_decalmaterials _decalnumtospawn _decalscale _fixeddecaloffset _decalmaxscale _decalminscale _decalrandomyaw _randomoffset) (break `DecalsProperties` (`self.DecalPropertiesConfig`)))
  ;[1 1 1] Set road painter decal properties variable (decals, scale, offset...)
  (for (_array_element _array_index) _decalmaterials
    (`KismetArrayLibrary.Array_Add` (`self.Decals Spawn`) (make `/Game/Carla/Blueprints/LevelDesign/RoadPaintDecals` _array_element (`|GetArrayItem` _decalnumtospawn _array_index)))
    (set `self.Decal scale` _decalscale)
    (set `self.Fixed decal offset` _fixeddecaloffset)
    (set `self.Decal max scale` _decalmaxscale)
    (set `self.Decal min scale` _decalminscale)
    (set `self.Decal Random Yaw` _decalrandomyaw)
    (set `self.Random Offset` _randomoffset)))

(event `Spawn decals`
  (bind _random_offset (`self.Random Offset`))
  (bind _returnvalue (`KismetMathLibrary.RandomFloatInRange` (* _random_offset -1.0) _random_offset))
  ;[1 1 1] Spawn decals
  (bind _returnvalue1 (`self.Load Waypoins from OD (Transform)` 500.0 :!label _label_2))
  (for (_ _array_index) (`self.Decals Spawn`)
    (bind (_decal _numberofdecals) (break `/Game/Carla/Blueprints/LevelDesign/RoadPaintDecals` (`|GetArrayItem` (`self.Decals Spawn`) _array_index)))
    (for _ (range 1 (+ _numberofdecals 1))
      (bind _returnvalue_2 (`self.Get any random points in the road` _returnvalue1))
      (bind _returnvalue_3 (`|SpawnActorFromClass` "/Script/Engine.DecalActor" (`KismetMathLibrary.MakeTransform` (+ (`self.Fixed decal offset`) (+ (.location _returnvalue_2) (`KismetMathLibrary.MakeVector` _returnvalue _returnvalue))) (`KismetMathLibrary.MakeRotator` (.roll (.rotation _returnvalue_2)) (.pitch (.rotation _returnvalue_2)) (+ (`KismetMathLibrary.RandomFloatInRange` 0.0 (`self.Decal Random Yaw`)) (.yaw (.rotation _returnvalue_2)))) (* (`self.Decal scale`) (`KismetMathLibrary.RandomFloatInRange` (`self.Decal min scale`) (`self.Decal max scale`)))) "Undefined" "OverrideRootScale" null null))
      (`DecalComponent.SetDecalMaterial` (`DecalActor.Decal` _returnvalue_3) _decal))))

(event `self.SpawnDecalsEvent`
  ;[1 1 1] Spawn decals
  (goto _label_2))

(fn `Get any random points in the road`
  (params (InputPin :type "Array of Transform Structure"))
  (returns (ReturnValue :type "Transform Structure"))
  (return (`|GetArrayItem` InputPin (`KismetMathLibrary.RandomIntegerInRange` 0 (`KismetArrayLibrary.Array_Length` InputPin)))))

(fn `Get sequence of locations`
  (returns (NewParam :type "Array of Vector Structure"))
  ;[1 1 1] Comment
  (bind _returnvalue (`self.Load Waypoins from OD (Location)` (`self.spacebeween brushes`)))
  (return _returnvalue))

(fn `Load Waypoins from OD (Location)`
  (params (ApproxDistance :type "Float (double-precision)"))
  (returns (ReturnValue :type "Array of Vector Structure"))
  (locals (NewLocalVar_0 :type "Waypoint Structure"))
  (bind _open_drive_map (`self.Open Drive Map`))
  (return (`OpenDriveMap.ComputeLocations` _open_drive_map (`OpenDriveMap.GenerateWaypoints` _open_drive_map ApproxDistance))))

(fn `Load Waypoins from OD (Transform)`
  (params (ApproxDistance :type "Float (double-precision)"))
  (returns (ReturnValue1 :type "Array of Transform Structure"))
  (bind _open_drive_map (`self.Open Drive Map`))
  (return (`OpenDriveMap.ComputeTransforms` _open_drive_map (`OpenDriveMap.GenerateWaypoints` _open_drive_map ApproxDistance))))

(fn `UserConstructionScript`
  (bind _returnvalue (`KismetMaterialLibrary.CreateDynamicMaterialInstance` (`self.Stencil`)))
  (set `self.RoadBrushMID` _returnvalue)
  (set `self.Open Drive Map` (`OpenDrive.LoadCurrentOpenDriveMap`)))